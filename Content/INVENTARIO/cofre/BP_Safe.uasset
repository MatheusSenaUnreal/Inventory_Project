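; BP_Safe is an interactable, passcode-locked safe that holds an inventory, showing an "OPEN SAFE" prompt and mesh highlight while the player overlaps it.
; Interacting opens W_Safe with the passcode and inventory component, while a looping timer polls its ABRIU flag.
; Once unlocked, it creates the chest inventory on the main HUD and swings the door with a Timeline.
; Another timer polls FecharBau to reverse the door and reset when that flag clears.
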(event `self.ReceiveBeginPlay`
  (bind _bpc_inventario (`self.BPC_Inventario`))
  (set `/Game/INVENTARIO/BPC_Inventario.Nome` (`self.Nome`) _bpc_inventario)
  (set `/Game/INVENTARIO/BPC_Inventario.SlotQuantidade` (`self.Slot Quantidade`) _bpc_inventario)
  (bind _asw_interact (cast `/Game/INVENTARIO/WIDGETS/W_Interact` (`WidgetComponent.GetWidget` (`self.Widget`))))
  (`TextBlock.SetText` (`/Game/INVENTARIO/WIDGETS/W_Interact.Nomedoitem` _asw_interact) (`KismetTextLibrary.Conv_NameToText` (`self.Nome`)))
  (`TextBlock.SetText` (`/Game/INVENTARIO/WIDGETS/W_Interact.quantidade` _asw_interact) "")
  (`TextBlock.SetText` (`/Game/INVENTARIO/WIDGETS/W_Interact.Raridade` _asw_interact) "")
  (`TextBlock.SetText` (`/Game/INVENTARIO/WIDGETS/W_Interact.Interragir` _asw_interact) "OPEN SAFE"))

(event `fechar bau`
  (bind _refmainhud (`/Game/INVENTARIO/BP_Controller.RefMainHud` (stale `AbrirCofre` _asbp_controller)))
  (bind _refbauinventario (`/Game/INVENTARIO/WIDGETS/W_MainHud.RefBauInventario` _refmainhud))
  (bind _fecharbau (`/Game/INVENTARIO/WIDGETS/W_BauInventario.FecharBau` _refbauinventario))
  (if _fecharbau :!label _label
    (bind (_direction _alpha) (`Timeline|Timeline` :!label _label_2)
      (:`Update`
        (`SceneComponent.K2_SetRelativeRotation` (`self.SafeDoor`) (`KismetMathLibrary.MakeRotator` 0.0 0.0 _alpha) false false)
        (if _fecharbau
          (bind _returnvalue (`KismetSystemLibrary.K2_SetTimerDelegate` (delegate `fechar bau`) 0.1 true))
          (set `self.Timer` _returnvalue)
          (else
            (`KismetSystemLibrary.K2_PauseTimerHandle` (`self.Timer`))
            (`KismetSystemLibrary.K2_PauseTimerHandle` (`self.Pause`))
            (goto _label_3 :!via `Reset`)))))
    (else
      (goto _label_2 :!via `ReverseFromEnd`))))

(event `AbrirCofre`
  (if (`/Game/INVENTARIO/WIDGETS/W_Safe.aBRIU` (`self.RefSafe`))
    (`/Engine/EditorBlueprintResources/StandardMacros.DoOnce` false :!label _label_3
      (:`Completed`
        (`Widget.RemoveFromParent` (`self.RefSafe`))
        (bind _asbp_controller (cast `/Game/INVENTARIO/BP_Controller` (`GameplayStatics.GetPlayerController` 0)))
        (bind _refmainhud (`/Game/INVENTARIO/BP_Controller.RefMainHud` _asbp_controller))
        (`/Game/INVENTARIO/WIDGETS/W_MainHud.Criar Bau Inventario` _refmainhud (`self.BPC_Inventario`))
        (set `/Game/INVENTARIO/WIDGETS/W_BauInventario.FecharBau` true (`/Game/INVENTARIO/WIDGETS/W_MainHud.RefBauInventario` _refmainhud))
        (goto _label)))))

(event `/Game/INVENTARIO/BPI_Interact.InteractItem`
  (params (Player :type "/Game/INVENTARIO/BP_Player Object Reference"))
  (bind _returnvalue (`GameplayStatics.GetPlayerController` 0))
  (bind _returnvalue_2 (`|CreateWidget` "/Game/INVENTARIO/WIDGETS/W_Safe.W_Safe_C" null (`self.Passe`) (`self.BPC_Inventario`)))
  (bind _output_get (set `self.RefSafe` _returnvalue_2))
  (`UserWidget.AddToViewport` _output_get 0)
  (`WidgetBlueprintLibrary.SetInputMode_UIOnlyEx` _returnvalue _output_get "DoNotLock" true)
  (set `PlayerController.bShowMouseCursor` true _returnvalue)
  (bind _returnvalue_3 (`KismetSystemLibrary.K2_SetTimerDelegate` (delegate `AbrirCofre`) 0.1 true))
  (set `self.Pause` _returnvalue_3))

(event `self.Sphere.OnComponentBeginOverlap`
  (params (OverlappedComponent :type "PrimitiveComponent Object Reference") (OtherActor :type "Actor Object Reference") (OtherComp :type "PrimitiveComponent Object Reference") (OtherBodyIndex :type Integer) (bFromSweep :type Boolean) (SweepResult :type "HitResult Structure (by ref)"))
  (cast `/Game/INVENTARIO/BP_Player` OtherActor)
  (`SceneComponent.SetVisibility` (`self.Widget`) true false)
  (`/Game/INVENTARIO/BP_Library.ItemHighLight` (`self.Safe`) true)
  (`/Game/INVENTARIO/BP_Library.ItemHighLight` (`self.SafeDoor`) true))

(event `self.Sphere.OnComponentEndOverlap`
  (params (OverlappedComponent :type "PrimitiveComponent Object Reference") (OtherActor :type "Actor Object Reference") (OtherComp :type "PrimitiveComponent Object Reference") (OtherBodyIndex :type Integer))
  (cast `/Game/INVENTARIO/BP_Player` OtherActor)
  (`SceneComponent.SetVisibility` (`self.Widget`) false false)
  (`/Game/INVENTARIO/BP_Library.ItemHighLight` (`self.Safe`))
  (`/Game/INVENTARIO/BP_Library.ItemHighLight` (`self.SafeDoor`)))

(fn `UserConstructionScript`)