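; BP_MasterMochil is a grabbable backpack pickup, apparently the master class for backpacks, passing its name and slot count to its inventory component.
; A sphere overlap with the player toggles the grab prompt widget and mesh highlight.
; Interacting drops any worn backpack at the player's DropLocation, then loops back to equip this one.
; Equipping copies the mesh onto MochilaAttach and parks the original, physics off, at a fixed world position instead of destroying it.
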(event `self.ReceiveBeginPlay`
  (bind _bpc_inventario (`self.BPC_Inventario`))
  (set `/Game/INVENTARIO/BPC_Inventario.Nome` (`self.Nome`) _bpc_inventario)
  (set `/Game/INVENTARIO/BPC_Inventario.SlotQuantidade` (`self.Slot Quantidade`) _bpc_inventario)
  (bind _asw_interact (cast `/Game/INVENTARIO/WIDGETS/W_Interact` (`WidgetComponent.GetWidget` (`self.Widget`))))
  (`TextBlock.SetText` (`/Game/INVENTARIO/WIDGETS/W_Interact.Nomedoitem` _asw_interact) (`KismetTextLibrary.Conv_NameToText` (`self.Nome`)))
  (`TextBlock.SetText` (`/Game/INVENTARIO/WIDGETS/W_Interact.quantidade` _asw_interact) "")
  (`TextBlock.SetText` (`/Game/INVENTARIO/WIDGETS/W_Interact.Raridade` _asw_interact) "")
  (`TextBlock.SetText` (`/Game/INVENTARIO/WIDGETS/W_Interact.Interragir` _asw_interact) "GRAB BACKPACK"))

(event `/Game/INVENTARIO/BPI_Interact.InteractItem`
  (params (Player :type "/Game/INVENTARIO/BP_Player Object Reference"))
  (bind _player (`self.Player`))
  (bind _asbp_controller (cast `/Game/INVENTARIO/BP_Controller` (`GameplayStatics.GetPlayerController` 0) :!pure true))
  (bind _returnvalue (`self.GetComponentByClass` (`/Game/INVENTARIO/BP_Player.Refmochila` _player) "/Script/Engine.StaticMeshComponent"))
  (set `self.Player` (cast `/Game/INVENTARIO/BP_Player` (`GameplayStatics.GetPlayerCharacter` 0) :!pure true))
  (if (`/Game/INVENTARIO/BP_Controller.Mochila?` _asbp_controller) :!label _label
    (set `/Game/INVENTARIO/BP_Controller.Mochila?` false _asbp_controller)
    (`SceneComponent.K2_SetWorldLocation` _returnvalue (`SceneComponent.K2_GetComponentLocation` (`/Game/INVENTARIO/BP_Player.DropLocation` (`self.Player`))) false true)
    (`KismetSystemLibrary.Delay` 0.01)
    (`PrimitiveComponent.SetSimulatePhysics` _returnvalue true)
    (goto _label)
    (else
      (bind _output_get (set `/Game/INVENTARIO/BP_Player.Refmochila` self _player))
      (set `/Game/INVENTARIO/BP_Controller.Mochila?` true (cast `/Game/INVENTARIO/BP_Controller` (`GameplayStatics.GetPlayerController` 0) :!pure true))
      (set `self.Static Mesh` (`StaticMeshComponent.StaticMesh` (`self.GetComponentByClass` _output_get "/Script/Engine.StaticMeshComponent")))
      (`StaticMeshComponent.SetStaticMesh` (`/Game/INVENTARIO/BP_Player.MochilaAttach` (`self.Player`)) (`self.Static Mesh`))
      (`SceneComponent.K2_SetWorldLocation` (`self.StaticMesh`) (0.0 0.0 1000.0) false false)
      (`PrimitiveComponent.SetSimulatePhysics` (`self.StaticMesh`) false))))

(event `self.Sphere.OnComponentBeginOverlap`
  (params (OverlappedComponent :type "PrimitiveComponent Object Reference") (OtherActor :type "Actor Object Reference") (OtherComp :type "PrimitiveComponent Object Reference") (OtherBodyIndex :type Integer) (bFromSweep :type Boolean) (SweepResult :type "HitResult Structure (by ref)"))
  (cast `/Game/INVENTARIO/BP_Player` OtherActor)
  (`SceneComponent.SetVisibility` (`self.Widget`) true false)
  (`/Game/INVENTARIO/BP_Library.ItemHighLight` (`self.StaticMesh`) true))

(event `self.Sphere.OnComponentEndOverlap`
  (params (OverlappedComponent :type "PrimitiveComponent Object Reference") (OtherActor :type "Actor Object Reference") (OtherComp :type "PrimitiveComponent Object Reference") (OtherBodyIndex :type Integer))
  (cast `/Game/INVENTARIO/BP_Player` OtherActor)
  (`SceneComponent.SetVisibility` (`self.Widget`) false false)
  (`/Game/INVENTARIO/BP_Library.ItemHighLight` (`self.StaticMesh`)))

(fn `UserConstructionScript`)