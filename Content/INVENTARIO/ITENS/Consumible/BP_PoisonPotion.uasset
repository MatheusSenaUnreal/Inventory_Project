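; BP_PoisonPotion is a consumable inventory item that poisons the player when used.
; UsarItem subtracts health from BP_Player immediately, then starts a one-second looping timer that calls DarDano.
; DarDano deals clamped damage each tick and uses a hit counter to pause the timer and reset after six ticks.
; Both events call the HUD health widget's update just before changing health, reached through BP_Controller.
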(event `self.UsarItem`
  (bind _asbp_player (cast `/Game/INVENTARIO/BP_Player` (`GameplayStatics.GetPlayerCharacter` 0) :!pure true))
  (`/Game/INVENTARIO/mainHudWidgtes/W_vida.AtualizarVida` (`/Game/INVENTARIO/WIDGETS/W_MainHud.W_vida` (`/Game/INVENTARIO/BP_Controller.RefMainHud` (cast `/Game/INVENTARIO/BP_Controller` (`GameplayStatics.GetPlayerController` 0) :!pure true))))
  (set `/Game/INVENTARIO/BP_Player.VidaAtual` (- (`/Game/INVENTARIO/BP_Player.VidaAtual` _asbp_player) 6.0) _asbp_player)
  (bind _returnvalue (`KismetSystemLibrary.K2_SetTimerDelegate` (delegate `DarDano`) 1.0 true))
  (`KismetSystemLibrary.PrintString` "VOCE USOU O ITEM"))

(event `DarDano`
  (bind _hit_damage_amount (`self.Hit Damage Amount`))
  (bind _asbp_player (cast `/Game/INVENTARIO/BP_Player` (`GameplayStatics.GetPlayerCharacter` 0) :!pure true))
  (`/Game/INVENTARIO/mainHudWidgtes/W_vida.AtualizarVida` (`/Game/INVENTARIO/WIDGETS/W_MainHud.W_vida` (`/Game/INVENTARIO/BP_Controller.RefMainHud` (cast `/Game/INVENTARIO/BP_Controller` (`GameplayStatics.GetPlayerController` 0) :!pure true))))
  (set `/Game/INVENTARIO/BP_Player.VidaAtual` (`KismetMathLibrary.FClamp` (- (`/Game/INVENTARIO/BP_Player.VidaAtual` _asbp_player) 6.0) 0.0 (`/Game/INVENTARIO/BP_Player.VidaMax` _asbp_player)) _asbp_player)
  (if (== _hit_damage_amount 5)
    (`KismetSystemLibrary.K2_PauseTimerHandle` (stale `self.UsarItem` _returnvalue))
    (set `self.Hit Damage Amount` 0)
    (else
      (`/Engine/EditorBlueprintResources/StandardMacros.IncrementInt` _hit_damage_amount))))

(fn `UserConstructionScript`
  (`parent.UserConstructionScript`))