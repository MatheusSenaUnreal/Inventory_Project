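; World item pickup whose mesh, name and rarity come from the class defaults of its item class, shown through an overlap-triggered widget and highlight.
; Interacting tries the player's hotbar, then inventory, then backpack if the controller flags one, keeping any leftover quantity or destroying itself.
; Inspect swaps input from player to item, moves it scaled down before the camera for mouse-drag rotation, and restores it on key 1.
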(event `/Game/INVENTARIO/BPI_Interact.InteractiTEM`
  (params (Player :type "/Game/INVENTARIO/BP_Player Object Reference"))
  (bind _bpc_inventario (`/Game/INVENTARIO/BP_Player.BPC_Inventario` (`self.Player`)))
  (bind _returnvalue (`self.GetComponentByClass` (`/Game/INVENTARIO/BP_Player.Refmochila` (`self.Player`)) "/Game/INVENTARIO/BPC_Inventario.BPC_Inventario_C"))
  (bind _output_get (set `self.Player` Player))
  (bind _hotbar (`/Game/INVENTARIO/BP_Player.hotbar` _output_get))
  (`/Engine/EditorBlueprintResources/StandardMacros.IsValid` _hotbar
    (:`Is Valid`
      (bind (_sucess_ _restodaquantidade) (`/Game/INVENTARIO/BPC_Inventario.AddItemAoInventario` _hotbar (`self.SouEsteItem`) (`self.Quantidade`)))
      (if _sucess_
        (if (> _restodaquantidade 0)
          (set `self.Quantidade` _restodaquantidade)
          (`self.Atualziar info interact`)
          (else
            (`self.K2_DestroyActor`)))
        (else
          (`/Engine/EditorBlueprintResources/StandardMacros.IsValid` _bpc_inventario
            (:`Is Valid`
              (bind (_sucess__2 _restodaquantidade_2) (`/Game/INVENTARIO/BPC_Inventario.AddItemAoInventario` _bpc_inventario (`self.SouEsteItem`) (`self.Quantidade`)))
              (if _sucess__2
                (if (> _restodaquantidade_2 0)
                  (set `self.Quantidade` _restodaquantidade_2)
                  (`self.Atualziar info interact`)
                  (else
                    (`self.K2_DestroyActor`)))
                (elif (`/Game/INVENTARIO/BP_Controller.Mochila?` (cast `/Game/INVENTARIO/BP_Controller` (`GameplayStatics.GetPlayerController` 0) :!pure true))
                  (`/Engine/EditorBlueprintResources/StandardMacros.IsValid` _returnvalue
                    (:`Is Valid`
                      (bind (_sucess__3 _restodaquantidade_3) (`/Game/INVENTARIO/BPC_Inventario.AddItemAoInventario` _returnvalue (`self.SouEsteItem`) (`self.Quantidade`)))
                      (if _sucess__3
                        (if (> _restodaquantidade_3 0)
                          (set `self.Quantidade` _restodaquantidade_3)
                          (`self.Atualziar info interact`)
                          (else
                            (`self.K2_DestroyActor`)))))))))))))))

(event `self.ReceiveBeginPlay`
  (bind ((`Nome_15_91F16EFA4D8B7D6B8F848B8B5B764866` _nome) (`Raridade_25_63001574434F0D98C18C7D9113E156CA` _raridade)) (break `/Game/INVENTARIO/STRUCT/ST_ItemStruct` (defaults `Object` (`self.SouEsteItem`))))
  (`StaticMeshComponent.SetStaticMesh` (`self.StaticMesh`) (`.Mesh_22_BB61F559402B6E8EA3415CBD7CB9B6EE` (break `/Game/INVENTARIO/STRUCT/ST_ItemStruct` (defaults `Object` (`self.SouEsteItem`)))) :!label _label)
  (bind _asw_interact (cast `/Game/INVENTARIO/WIDGETS/W_Interact` (`WidgetComponent.GetWidget` (`self.Widget`))))
  (bind _output_get (set `self.Ref W Interact` _asw_interact))
  (`TextBlock.SetText` (`/Game/INVENTARIO/WIDGETS/W_Interact.Nomedoitem` _output_get) (`KismetTextLibrary.Conv_NameToText` _nome))
  (`TextBlock.SetText` (`/Game/INVENTARIO/WIDGETS/W_Interact.quantidade` _output_get) (`KismetTextLibrary.Conv_IntToText` (`self.Quantidade`)))
  (`TextBlock.SetText` (`/Game/INVENTARIO/WIDGETS/W_Interact.Raridade` _output_get) (`KismetTextLibrary.Conv_StringToText` (`|GetEnumeratorNameAsString` _raridade)))
  (`TextBlock.SetText` (`/Game/INVENTARIO/WIDGETS/W_Interact.Interragir` _output_get) "PICK UP ITEM")
  (`self.MudarCorRaridade`))

(event `Atualziar info interact`
  (goto _label))

(event `self.Sphere.OnComponentBeginOverlap`
  (params (OverlappedComponent :type "PrimitiveComponent Object Reference") (OtherActor :type "Actor Object Reference") (OtherComp :type "PrimitiveComponent Object Reference") (OtherBodyIndex :type Integer) (bFromSweep :type Boolean) (SweepResult :type "HitResult Structure (by ref)"))
  (cast `/Game/INVENTARIO/BP_Player` OtherActor)
  (`SceneComponent.SetVisibility` (`self.Widget`) true false)
  (`/Game/INVENTARIO/BP_Library.ItemHighLight` (`self.StaticMesh`) true))

(event `self.Sphere.OnComponentEndOverlap`
  (params (OverlappedComponent :type "PrimitiveComponent Object Reference") (OtherActor :type "Actor Object Reference") (OtherComp :type "PrimitiveComponent Object Reference") (OtherBodyIndex :type Integer))
  (cast `/Game/INVENTARIO/BP_Player` OtherActor)
  (`SceneComponent.SetVisibility` (`self.Widget`) false false)
  (`/Game/INVENTARIO/BP_Library.ItemHighLight` (`self.StaticMesh`)))

(event `/Game/INVENTARIO/BPI_Interact.Inspect`
  (params (Player :type "/Game/INVENTARIO/BP_Player Object Reference"))
  (bind _output_get (set `self.Player` Player))
  (`/Game/INVENTARIO/BP_Player.ItemAtual` _output_get
    (:`then`)
    (:`else`
      (`self.StartInspect`)
      (`KismetSystemLibrary.PrintString` "111Hello"))))

(event `Key|One`
  (params (Key :type "Key Structure"))
  (:`Pressed`
    (`self.StopInsect`)
    (set `/Game/INVENTARIO/BP_Player.ItemAtual` null (stale `/Game/INVENTARIO/BPI_Interact.Inspect` _output_get))))

(event `Key|LeftMouseButton`
  (params (Key :type "Key Structure"))
  (:`Pressed`
    (set `self.NewVar_0` true))
  (:`Released`
    (set `self.NewVar_0` false)))

(event `InputAxisKey|MouseX`
  (params (AxisValue :type "Float (single-precision)"))
  (if (`self.NewVar_0`)
    (`self.K2_SetActorRotation` (`KismetMathLibrary.ComposeRotators` (`self.K2_GetActorRotation`) (`KismetMathLibrary.MakeRotator` 0.0 0.0 (* AxisValue 3.0))))))

(event `InputAxisKey|MouseY`
  (params (AxisValue :type "Float (single-precision)"))
  (if (`self.NewVar_0`)
    (`self.K2_SetActorRotation` (`KismetMathLibrary.ComposeRotators` (`self.K2_GetActorRotation`) (`KismetMathLibrary.MakeRotator` 0.0 (* AxisValue 3.0))))))

(fn `Cores`
  (params (Text :type "TextBlock Object Reference"))
  (returns (Comum :type "SlateColor Structure") (Incomum :type "SlateColor Structure") (Raro :type "SlateColor Structure") (`Muito-Raro` :type "SlateColor Structure") (Epico :type "SlateColor Structure") (Lendario :type "SlateColor Structure") (Mitico :type "SlateColor Structure"))
  (return (`self.Cor Comum`) (`self.Cor Incomum`) (`self.Cor Raro`) (`self.Cor Muito- Raro`) (`self.Cor Epico`) (`self.Cor Lendario`) (`self.Cor Mitico`)))

(fn `MudarCorRaridade`
  (bind _raridade (`/Game/INVENTARIO/WIDGETS/W_Interact.Raridade` (`self.Ref W Interact`)))
  (switch `/Game/INVENTARIO/enum/E_Raridade` (`.Raridade_25_63001574434F0D98C18C7D9113E156CA` (break `/Game/INVENTARIO/STRUCT/ST_ItemStruct` (defaults `Object` (`self.SouEsteItem`))))
    (:`NewEnumerator0`
      (bind _comum (`self.Cores` _raridade))
      (`TextBlock.SetColorAndOpacity` _raridade _comum)
      (`TextBlock.SetText` _raridade "Common"))
    (:`NewEnumerator1`
      (bind (_comum_2 _incomum) (`self.Cores` _raridade))
      (`TextBlock.SetColorAndOpacity` _raridade _incomum)
      (`TextBlock.SetText` _raridade "Uncommon"))
    (:`NewEnumerator2`
      (bind (_comum_3 _incomum_2 _raro) (`self.Cores` _raridade))
      (`TextBlock.SetColorAndOpacity` _raridade _raro)
      (`TextBlock.SetText` _raridade "Raro"))
    (:`NewEnumerator3`
      (bind (_comum_4 _incomum_3 _raro_2 _muito_raro) (`self.Cores` _raridade))
      (`TextBlock.SetColorAndOpacity` _raridade _muito_raro)
      (`TextBlock.SetText` _raridade "Very-Rare"))
    (:`NewEnumerator4`
      (bind (_comum_5 _incomum_4 _raro_3 _muito_raro_2 _epico) (`self.Cores` _raridade))
      (`TextBlock.SetColorAndOpacity` _raridade _epico)
      (`TextBlock.SetText` _raridade "Epic"))
    (:`NewEnumerator5`
      (bind (_comum_6 _incomum_5 _raro_4 _muito_raro_3 _epico_2 _lendario) (`self.Cores` _raridade))
      (`TextBlock.SetColorAndOpacity` _raridade _lendario)
      (`TextBlock.SetText` _raridade "Legendary"))
    (:`NewEnumerator6`
      (bind (_comum_7 _incomum_6 _raro_5 _muito_raro_4 _epico_3 _lendario_2 _mitico) (`self.Cores` _raridade))
      (`TextBlock.SetColorAndOpacity` _raridade _mitico)
      (`TextBlock.SetText` _raridade "Mythical"))))

(fn `StartInspect`
  (bind _returnvalue (`GameplayStatics.GetPlayerCameraManager` 0))
  (bind _returnvalue_2 (`GameplayStatics.GetPlayerController` 0))
  (bind _player (`self.Player`))
  (bind _returnvalue_3 (+ (`PlayerCameraManager.GetCameraLocation` _returnvalue) (* (`KismetMathLibrary.GetForwardVector` (`PlayerCameraManager.GetCameraRotation` _returnvalue)) (`self.NewVar`))))
  (set `self.NewVar_1` (`self.GetTransform`))
  (`self.DisableInput` _player _returnvalue_2)
  (`self.EnableInput` _returnvalue_2)
  (`self.K2_AttachToComponent` (`/Game/INVENTARIO/BP_Player.Scene` _player) "None" "SnapToTarget" "SnapToTarget" "KeepRelative")
  (set `/Game/INVENTARIO/BP_Player.ItemAtual` self (`self.Player`))
  (set `self.NewVar_2` _returnvalue_3)
  (`self.K2_SetActorLocation` (`KismetMathLibrary.MakeVector` (.x _returnvalue_3) (.y _returnvalue_3) (- (.z _returnvalue_3) 5.0)))
  (`self.SetActorScale3D` (0.1 0.1 0.1)))

(fn `StopInsect`
  (bind _returnvalue (`GameplayStatics.GetPlayerController` 0))
  (bind (_newvar_1_location _newvar_1_rotation _newvar_1_scale) (`KismetMathLibrary.BreakTransform` (`self.NewVar_1`)))
  (`self.DisableInput` _returnvalue)
  (`self.EnableInput` (`self.Player`) _returnvalue)
  (`self.K2_SetActorTransform` (`KismetMathLibrary.MakeTransform` _newvar_1_location _newvar_1_rotation _newvar_1_scale))
  (`self.K2_DetachFromActor` "KeepWorld" "KeepWorld" "KeepWorld"))

(fn `UserConstructionScript`
  (`StaticMeshComponent.SetStaticMesh` (`self.StaticMesh`) (`.Mesh_22_BB61F559402B6E8EA3415CBD7CB9B6EE` (break `/Game/INVENTARIO/STRUCT/ST_ItemStruct` (defaults `Object` (`self.SouEsteItem`))))))