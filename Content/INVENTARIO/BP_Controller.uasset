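; BP_Controller is the controller that sets up the player's main HUD and opens the inventory UI.
; On BeginPlay it creates W_MainHud, adds it to the viewport and caches a reference to the BP_Player character.
; Pressing Tab checks the Mochila flag to have the HUD create either the backpack inventory, using the BPC_Inventario component from the player's backpack reference, or the standard inventory.
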(event `self.ReceiveBeginPlay`
  (bind _returnvalue (`|CreateWidget` "/Game/INVENTARIO/WIDGETS/W_MainHud.W_MainHud_C"))
  (bind _output_get (set `self.RefMainHud` _returnvalue))
  (`UserWidget.AddToViewport` _output_get 0)
  (bind _asbp_player (cast `/Game/INVENTARIO/BP_Player` (`GameplayStatics.GetPlayerCharacter` 0)))
  (set `self.RefPlayer` _asbp_player))

(event `Key|Tab`
  (params (Key :type "Key Structure"))
  (bind _refmainhud (`self.RefMainHud`))
  (:`Pressed`
    (if (`self.Mochila?`)
      (`/Game/INVENTARIO/WIDGETS/W_MainHud.CriarMochilainventario` _refmainhud (`self.GetComponentByClass` (`/Game/INVENTARIO/BP_Player.Refmochila` (`self.RefPlayer`)) "/Game/INVENTARIO/BPC_Inventario.BPC_Inventario_C"))
      (else
        (`/Game/INVENTARIO/WIDGETS/W_MainHud.Criar Inventario` _refmainhud)))))

(fn `UserConstructionScript`)