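; BP_Bau is an interactable chest with its own inventory component, configured from its name and slot count.
; A sphere overlap with the player toggles the "OPEN CHEST" prompt widget and highlights the body and lid.
; InteractItem creates the chest inventory on the main HUD and starts the lid timeline.
; A looping timer set from the timeline update polls the UI's FecharBau flag, reversing the lid when it turns false.
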(event `self.ReceiveBeginPlay`
  (bind _bpc_inventario (`self.BPC_Inventario`))
  (set `/Game/INVENTARIO/BPC_Inventario.Nome` (`self.Nome`) _bpc_inventario)
  (set `/Game/INVENTARIO/BPC_Inventario.SlotQuantidade` (`self.Slot Quantidade`) _bpc_inventario)
  (bind _asw_interact (cast `/Game/INVENTARIO/WIDGETS/W_Interact` (`WidgetComponent.GetWidget` (`self.Widget`))))
  (`TextBlock.SetText` (`/Game/INVENTARIO/WIDGETS/W_Interact.Nomedoitem` _asw_interact) (`KismetTextLibrary.Conv_NameToText` (`self.Nome`)))
  (`TextBlock.SetText` (`/Game/INVENTARIO/WIDGETS/W_Interact.quantidade` _asw_interact) "")
  (`TextBlock.SetText` (`/Game/INVENTARIO/WIDGETS/W_Interact.Raridade` _asw_interact) "")
  (`TextBlock.SetText` (`/Game/INVENTARIO/WIDGETS/W_Interact.Interragir` _asw_interact) "OPEN CHEST"))

(event `fechar bau`
  (bind _fecharbau (`/Game/INVENTARIO/WIDGETS/W_BauInventario.FecharBau` (`/Game/INVENTARIO/WIDGETS/W_MainHud.RefBauInventario` (`/Game/INVENTARIO/BP_Controller.RefMainHud` (stale `/Game/INVENTARIO/BPI_Interact.InteractItem` _asbp_controller)))))
  (if _fecharbau :!label _label
    (bind (_direction _alpha) (`Timeline|Timeline` :!label _label_2)
      (:`Update`
        (`SceneComponent.K2_SetRelativeRotation` (`self.BauTampa`) (`KismetMathLibrary.MakeRotator` _alpha) false false)
        (if _fecharbau
          (bind _returnvalue (`KismetSystemLibrary.K2_SetTimerDelegate` (delegate `fechar bau`) 0.1 true))
          (set `self.Timer` _returnvalue)
          (else
            (`KismetSystemLibrary.K2_PauseTimerHandle` (`self.Timer`))))))
    (else
      (goto _label_2 :!via `ReverseFromEnd`))))

(event `/Game/INVENTARIO/BPI_Interact.InteractItem`
  (params (Player :type "/Game/INVENTARIO/BP_Player Object Reference"))
  (bind _asbp_controller (cast `/Game/INVENTARIO/BP_Controller` (`GameplayStatics.GetPlayerController` 0)))
  (bind _refmainhud (`/Game/INVENTARIO/BP_Controller.RefMainHud` _asbp_controller))
  (`/Game/INVENTARIO/WIDGETS/W_MainHud.Criar Bau Inventario` _refmainhud (`self.BPC_Inventario`))
  (set `/Game/INVENTARIO/WIDGETS/W_BauInventario.FecharBau` true (`/Game/INVENTARIO/WIDGETS/W_MainHud.RefBauInventario` _refmainhud))
  (goto _label))

(event `self.Sphere.OnComponentBeginOverlap`
  (params (OverlappedComponent :type "PrimitiveComponent Object Reference") (OtherActor :type "Actor Object Reference") (OtherComp :type "PrimitiveComponent Object Reference") (OtherBodyIndex :type Integer) (bFromSweep :type Boolean) (SweepResult :type "HitResult Structure (by ref)"))
  (cast `/Game/INVENTARIO/BP_Player` OtherActor)
  (`SceneComponent.SetVisibility` (`self.Widget`) true false)
  (`/Game/INVENTARIO/BP_Library.ItemHighLight` (`self.Bau`) true)
  (`/Game/INVENTARIO/BP_Library.ItemHighLight` (`self.BauTampa`) true))

(event `self.Sphere.OnComponentEndOverlap`
  (params (OverlappedComponent :type "PrimitiveComponent Object Reference") (OtherActor :type "Actor Object Reference") (OtherComp :type "PrimitiveComponent Object Reference") (OtherBodyIndex :type Integer))
  (cast `/Game/INVENTARIO/BP_Player` OtherActor)
  (`SceneComponent.SetVisibility` (`self.Widget`) false false)
  (`/Game/INVENTARIO/BP_Library.ItemHighLight` (`self.Bau`))
  (`/Game/INVENTARIO/BP_Library.ItemHighLight` (`self.BauTampa`)))

(fn `UserConstructionScript`)