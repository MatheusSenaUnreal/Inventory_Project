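; Inventory component holding a fixed-size array of item class and quantity slots, with item data read from class defaults.
; AddItemAoInventario fills a matching stack or empty slot, recursing on overflow and returning any leftover quantity.
; MudarSlot merges or swaps slots and DividirPilha halves a stack into an empty slot, both across components, then fire AtualizarTrocaDeSlot on each.
; DepositarItemRapido and the Tab-triggered SetColl are empty.
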(event `self.ReceiveBeginPlay`
  (`KismetArrayLibrary.Array_Resize` (`self.Inventario`) (`self.SlotQuantidade`)))

(event `Key|Tab`
  (params (Key :type "Key Structure"))
  (:`Pressed`
    (`self.SetColl`)))

(event `SetColl`)

(event `AtualizarTrocaDeSlot`
  (`self.AtualizarInventario`))

(fn `AddItemAoInventario`
  (params (Item :type "/Game/INVENTARIO/ITENS/BP_ItemMaster Class Reference") (Quantidad :type Integer))
  (returns (`Sucess?` :type Boolean) (RestoDaQuantidade :type Integer))
  (locals (LocalItem :type "/Game/INVENTARIO/ITENS/BP_ItemMaster Class Reference") (LocalQuantidade :type Integer) (LocalEmpilhamnetoMax :type Integer) (`LocalIndeItem/Pilha` :type Integer))
  (bind ((`MaxStack_17_3F5DA89C47D4BC78D7455A8771DBB47B` _maxstack) (`Empilhavel?_12_4933F3AD41DDF44D6D73BEA7F2115FA6` _empilhavel_)) (break `/Game/INVENTARIO/STRUCT/ST_ItemStruct` (defaults `Object` Item)))
  (bind _returnvalue (+ (`.Quantidade_5_2CDF2731400EA3EE6641069DF4103200` (break `/Game/INVENTARIO/STRUCT/ST_SlotInventario` (`|GetArrayItem` (`self.Inventario`) (`local.LocalIndeItem/Pilha`)))) (`local.LocalQuantidade`)))
  (set `local.LocalItem` Item)
  (set `local.LocalQuantidade` Quantidad)
  (set `local.LocalEmpilhamnetoMax` _maxstack)
  (if _empilhavel_
    (bind (_pilhaencotrada _indexdapilha) (`self.ProcurarEmpilhamento` (`local.LocalItem`)))
    (if _pilhaencotrada
      (set `local.LocalIndeItem/Pilha` _indexdapilha)
      (if (> _returnvalue (`local.LocalEmpilhamnetoMax`))
        (set `local.LocalQuantidade` (- _returnvalue (`local.LocalEmpilhamnetoMax`)))
        (`KismetArrayLibrary.Array_Set` (`self.Inventario`) (`local.LocalIndeItem/Pilha`) (make `/Game/INVENTARIO/STRUCT/ST_SlotInventario` (`local.LocalItem`) (`local.LocalEmpilhamnetoMax`))) ; SE ESSA SOMA FOR MAIOR QUE O EMPILHAMENTO\nMAXIMO DESSE ITEM, ELE VAI SETAR O VALOR MAXIMO\nNESSA PILHA E PROCURAR OUTRO SLOT PARA O QUE SOBROU
        (bind (_sucess_ _restodaquantidade) (`self.AddItemAoInventario` (`local.LocalItem`) (`local.LocalQuantidade`)))
        (return true _restodaquantidade)
        (else
          (`KismetArrayLibrary.Array_Set` (`self.Inventario`) (`local.LocalIndeItem/Pilha`) (make `/Game/INVENTARIO/STRUCT/ST_SlotInventario` (`local.LocalItem`) _returnvalue))
          (return true 0) ; SE N FOR MAIOR VAI SETAR O RESULTADO DA SOMA\nNO SLOT
        ))
      (else
        (bind (_slotfreesetado _indexfreesetado) (`self.ProcurarSlotVazio`))
        (if _slotfreesetado
          (set `local.LocalIndeItem/Pilha` _indexfreesetado)
          (if (> (`local.LocalQuantidade`) (`local.LocalEmpilhamnetoMax`))
            (`KismetArrayLibrary.Array_Set` (`self.Inventario`) (`local.LocalIndeItem/Pilha`) (make `/Game/INVENTARIO/STRUCT/ST_SlotInventario` (`local.LocalItem`) (`local.LocalEmpilhamnetoMax`))) ; SE FOR MAIOR QUE O STACK MAXIMO SETAMOS O PROPRIO\nSTACK MAXIMO NESSE SLOT E PROCURAMOS OUTRO SLOT \nPARA O QUE SOBROU
            (bind (_sucess__2 _restodaquantidade_2) (`self.AddItemAoInventario` (`local.LocalItem`) (- (`local.LocalQuantidade`) (`local.LocalEmpilhamnetoMax`))))
            (return true _restodaquantidade_2) ; SOBROU QUANTIDADE?
            (else
              (`KismetArrayLibrary.Array_Set` (`self.Inventario`) (`local.LocalIndeItem/Pilha`) (make `/Game/INVENTARIO/STRUCT/ST_SlotInventario` (`local.LocalItem`) (`local.LocalQuantidade`)))
              (return true 0) ; SE N FOR SETA  QUANTIDADE DELE NO SLOT LIVRE
            ))
          (else
            (return false (`local.LocalQuantidade`))))))
    (else
      (bind (_slotfreesetado_2 _indexfreesetado_2) (`self.ProcurarSlotVazio`))
      (if _slotfreesetado_2
        (bind _output_get (set `local.LocalIndeItem/Pilha` _indexfreesetado_2))
        (`KismetArrayLibrary.Array_Set` (`self.Inventario`) _output_get (make `/Game/INVENTARIO/STRUCT/ST_SlotInventario` (`local.LocalItem`) 1)) ; SETANDO NO INVENTARIO
        (if (> (`local.LocalQuantidade`) 1)
          (bind (_sucess__3 _restodaquantidade_3) (`self.AddItemAoInventario` (`local.LocalItem`) (- (`local.LocalQuantidade`) 1))) ; SE TVER ELE ADD O ITEM SUBTRAINDO O QUE ESTA NO CHAO
          (return true _restodaquantidade_3)
          (else
            (return true 0)))
        (else
          (return false (`local.LocalQuantidade`)) ; SE N ACHAR VAI DEIXAR A\nQUANTIDADE DESSE ITEM\nNO CHAO
        )))))

(fn `DepositarItemRapido`
  (params (IndexDe :type Integer) (IndexPara :type Integer) (BPCinventario :type "/Game/INVENTARIO/BPC_Inventario Object Reference")))

(fn `DividirPilha`
  (params (IndexDe :type Integer) (IndexPara :type Integer) (BPCinventario :type "/Game/INVENTARIO/BPC_Inventario Object Reference"))
  (locals (LocalIndexParaa :type Integer :default 0) (LocalIndexDe :type Integer :default 0) (LocalSlotInfo :type "/Game/INVENTARIO/STRUCT/ST_SlotInventario Structure") (LocalQuantidade :type Integer :default 0) (LocalItemClass :type "/Game/INVENTARIO/ITENS/BP_ItemMaster Class Reference"))
  (bind _localquantidade (`local.LocalQuantidade`))
  (bind _returnvalue (/ _localquantidade 2))
  (bind _output (`|GetArrayItem` (`/Game/INVENTARIO/BPC_Inventario.Inventario` (`local.BPCinventario`)) (`local.LocalIndexDe`)))
  (bind (_iteminfo _quantidade) (break `/Game/INVENTARIO/STRUCT/ST_SlotInventario` _output))
  (set `local.LocalIndexDe` IndexDe)
  (set `local.LocalIndexParaa` IndexPara)
  (bind _output_get (set `local.LocalQuantidade` _quantidade))
  (if (> _output_get 1)
    (set `local.LocalSlotInfo` _output)
    (set `local.LocalItemClass` _iteminfo)
    (if (not (`KismetSystemLibrary.IsValidClass` (`.ItemInfo_6_91F16EFA4D8B7D6B8F848B8B5B764866` (break `/Game/INVENTARIO/STRUCT/ST_SlotInventario` (`|GetArrayItem` (`self.Inventario`) (`local.LocalIndexParaa`))))))
      (`KismetArrayLibrary.Array_Set` (`/Game/INVENTARIO/BPC_Inventario.Inventario` (`local.BPCinventario`)) (`local.LocalIndexDe`) (make `/Game/INVENTARIO/STRUCT/ST_SlotInventario` (`local.LocalItemClass`) _returnvalue))
      (if (== (`KismetMathLibrary.And_IntInt` _localquantidade 1) 1)
        (`KismetArrayLibrary.Array_Set` (`self.Inventario`) (`local.LocalIndexParaa`) (make `/Game/INVENTARIO/STRUCT/ST_SlotInventario` (`local.LocalItemClass`) (+ _returnvalue 1)))
        (else
          (`KismetArrayLibrary.Array_Set` (`self.Inventario`) (`local.LocalIndexParaa`) (make `/Game/INVENTARIO/STRUCT/ST_SlotInventario` (`local.LocalItemClass`) _returnvalue))))
      (`self.AtualizarTrocaDeSlot`)
      (`self.AtualizarTrocaDeSlot` (`local.BPCinventario`)))))

(fn `MudarSlot`
  (params (IndexDe :type Integer) (IndexPara :type Integer) (BPCinventario :type "/Game/INVENTARIO/BPC_Inventario Object Reference"))
  (locals (LocalIndexParaa :type Integer :default 0) (LocalIndexDe :type Integer :default 0) (LocalSlotInfo :type "/Game/INVENTARIO/STRUCT/ST_SlotInventario Structure") (LocalResSoma :type Integer) (LocalMaxStack :type Integer) (LocalItemClass :type "/Game/INVENTARIO/ITENS/BP_ItemMaster Class Reference"))
  (bind (_iteminfo _quantidade) (break `/Game/INVENTARIO/STRUCT/ST_SlotInventario` (`local.LocalSlotInfo`)))
  (bind ((`MaxStack_17_3F5DA89C47D4BC78D7455A8771DBB47B` _maxstack) (`Empilhavel?_12_4933F3AD41DDF44D6D73BEA7F2115FA6` _empilhavel_)) (break `/Game/INVENTARIO/STRUCT/ST_ItemStruct` (defaults `Object` (`local.LocalItemClass`))))
  (bind (_iteminfo_2 _quantidade_2) (break `/Game/INVENTARIO/STRUCT/ST_SlotInventario` (`|GetArrayItem` (`self.Inventario`) (`local.IndexPara`))))
  (set `local.LocalIndexDe` IndexDe)
  (set `local.LocalIndexParaa` IndexPara)
  (set `local.LocalSlotInfo` (`|GetArrayItem` (`/Game/INVENTARIO/BPC_Inventario.Inventario` (`local.BPCinventario`)) (`local.LocalIndexDe`)))
  (set `local.LocalItemClass` _iteminfo)
  (set `local.LocalResSoma` (+ _quantidade _quantidade_2))
  (bind _output_get (set `local.LocalMaxStack` _maxstack))
  (if (== (`local.LocalItemClass`) _iteminfo_2)
    (if _empilhavel_
      (if (< (`local.LocalResSoma`) _output_get)
        (`KismetArrayLibrary.Array_Set` (`/Game/INVENTARIO/BPC_Inventario.Inventario` (`local.BPCinventario`)) (`local.IndexDe`) (make `/Game/INVENTARIO/STRUCT/ST_SlotInventario` (`local.LocalItemClass`)))
        (`KismetArrayLibrary.Array_Set` (`self.Inventario`) (`local.IndexPara`) (make `/Game/INVENTARIO/STRUCT/ST_SlotInventario` (`local.LocalItemClass`) (`local.LocalResSoma`)))
        (else
          (`KismetArrayLibrary.Array_Set` (`/Game/INVENTARIO/BPC_Inventario.Inventario` (`local.BPCinventario`)) (`local.IndexDe`) (make `/Game/INVENTARIO/STRUCT/ST_SlotInventario` (`local.LocalItemClass`) (- (`local.LocalResSoma`) (`local.LocalMaxStack`))))
          (`KismetArrayLibrary.Array_Set` (`self.Inventario`) (`local.IndexPara`) (make `/Game/INVENTARIO/STRUCT/ST_SlotInventario` (`local.LocalItemClass`) (`local.LocalMaxStack`)))))
      (`self.AtualizarTrocaDeSlot` :!label _label)
      (`self.AtualizarTrocaDeSlot` (`local.BPCinventario`)))
    (else
      (`KismetArrayLibrary.Array_Set` (`/Game/INVENTARIO/BPC_Inventario.Inventario` (`local.BPCinventario`)) (`local.IndexDe`) (`|GetArrayItem` (`self.Inventario`) (`local.IndexPara`)))
      (`KismetArrayLibrary.Array_Set` (`self.Inventario`) (`local.IndexPara`) (`local.LocalSlotInfo`))
      (goto _label))))

(fn `PegarInfoDoItemIndex`
  (params (Index :type Integer))
  (returns (`SlotFree?` :type Boolean) (Quantidade :type Integer) (ItemInfo :type "/Game/INVENTARIO/STRUCT/ST_ItemStruct Structure"))
  (bind (_iteminfo _quantidade) (break `/Game/INVENTARIO/STRUCT/ST_SlotInventario` (`|GetArrayItem` (`self.Inventario`) Index)))
  (if (`KismetSystemLibrary.IsValidClass` _iteminfo)
    (return false _quantidade (defaults `Object` _iteminfo))
    (else
      (return true 0))))

(fn `ProcurarEmpilhamento`
  (params (Item :type "/Game/INVENTARIO/ITENS/BP_ItemMaster Class Reference"))
  (returns (PilhaEncotrada :type Boolean) (IndexDaPilha :type Integer))
  (locals (LocalPilhaEncotrada :type Boolean :default false) (LocalIndexDaPilha :type Integer :default 0))
  (for (_array_element _array_index) (`self.Inventario`)
    (bind (_iteminfo _quantidade) (break `/Game/INVENTARIO/STRUCT/ST_SlotInventario` _array_element))
    (if (`KismetSystemLibrary.IsValidClass` _iteminfo)
      (if (and (== _iteminfo (`local.Item`)) (< _quantidade (`.MaxStack_17_3F5DA89C47D4BC78D7455A8771DBB47B` (break `/Game/INVENTARIO/STRUCT/ST_ItemStruct` (defaults `Object` Item)))))
        (set `local.LocalPilhaEncotrada` true)
        (set `local.LocalIndexDaPilha` _array_index)
        (break))))
  (return (`local.LocalPilhaEncotrada`) (`local.LocalIndexDaPilha`)) ; VAI ARMAZENAR O VALOR ENCOTRADO
)

(fn `ProcurarSlotVazio`
  (returns (SlotFreeSetado :type Boolean) (IndexFreeSetado :type Integer))
  (locals (`LocalSlotFree?` :type Boolean :default false) (LocalIndexFree :type Integer :default 0))
  (for (_array_element _array_index) (`self.Inventario`)
    (if (not (`KismetSystemLibrary.IsValidClass` (`.ItemInfo_6_91F16EFA4D8B7D6B8F848B8B5B764866` (break `/Game/INVENTARIO/STRUCT/ST_SlotInventario` _array_element))))
      (set `local.LocalSlotFree?` true)
      (set `local.LocalIndexFree` _array_index)
      (break)))
  (return (`local.LocalSlotFree?`) (`local.LocalIndexFree`)) ; VAI GUARDAR A INFO DO SLOT VAZIO ENCOTRADO
)